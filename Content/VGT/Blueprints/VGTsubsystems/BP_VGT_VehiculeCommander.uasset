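; BP_VGT_VehiculeCommander adds mouse-wheel camera zoom for the vehicle referenced by its ACVGTGravityComponent.
; On BeginPlay it retries on a short delay until that component is valid, then enables input for the component's PlayerController and caches the vehicle's SpringArm.
; Wheel up and down shorten or lengthen the arm in fixed, unclamped steps.
; The MouseY axis event only checks the arm's validity and does nothing further.
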(event EventBeginPlay
  (bind _ac_vgt_gravitycomponent (Variables|Default|GetAC_VGT_GravityComponent))
  (bind _ac_vgt_gravitycomponent_2 (Variables|Default|GetAC_VGT_GravityComponent))
  (bind _vehicule (Variables|/Game/VGT/Blueprints/AC_VGT_GravityComponent.AC_VGT_GravityComponent_C|GetVehicule _ac_vgt_gravitycomponent_2))
  (bind _returnvalue (Actor|GetComponentbyClass _vehicule "/Script/Engine.SpringArmComponent"))
  (Utilities|IsValid _ac_vgt_gravitycomponent :!label _label
    (:Is%20Valid
      (Input|EnableInput (Variables|/Game/VGT/Blueprints/AC_VGT_GravityComponent.AC_VGT_GravityComponent_C|GetPlayerController _ac_vgt_gravitycomponent))
      (Utilities|IsValid _returnvalue
        (:Is%20Valid
          (Variables|Default|SetSpringArm _returnvalue))))
    (:Is%20Not%20Valid
      (Utilities|FlowControl|Delay 0.1)
      (goto _label))))

(event Input|MouseEvents|MouseY
  (params (AxisValue :type Float%20%28single-precision%29))
  (Utilities|IsValid (Variables|Default|GetSpringArm)))

(event Input|MouseEvents|MouseWheelUp
  (params (Key :type Key%20Structure))
  (bind _springarm (Variables|Default|GetSpringArm))
  (:Pressed
    (Utilities|IsValid _springarm
      (:Is%20Valid
        (Variables|/Script/Engine.SpringArmComponent|SetTargetArmLength _springarm (- (Variables|/Script/Engine.SpringArmComponent|GetTargetArmLength _springarm) 1e+02))))))

(event Input|MouseEvents|MouseWheelDown
  (params (Key :type Key%20Structure))
  (bind _springarm (Variables|Default|GetSpringArm))
  (:Pressed
    (Utilities|IsValid _springarm
      (:Is%20Valid
        (Variables|/Script/Engine.SpringArmComponent|SetTargetArmLength _springarm (+ (Variables|/Script/Engine.SpringArmComponent|GetTargetArmLength _springarm) 1e+02))))))

(fn ConstructionScript)